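; BP_Turret is a turret that lets the player switch between four gun types with number keys.
; Keys 1 to 4 swap the class of the TurretGun child actor component to the standard, double-barreled, laser or arc gun Blueprint.
; BeginPlay shows the mouse cursor, and this graph holds no aiming or firing logic.
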(event `self.ReceiveBeginPlay`
  (set `PlayerController.bShowMouseCursor` true (`GameplayStatics.GetPlayerController` 0)))

(event `Key|One`
  (params (Key :type "Key Structure"))
  (:`Pressed`
    (`ChildActorComponent.SetChildActorClass` (`self.TurretGun`) "/Game/Gun/BP_StandardGun.BP_StandardGun_C")))

(event `Key|Two`
  (params (Key :type "Key Structure"))
  (:`Pressed`
    (`ChildActorComponent.SetChildActorClass` (`self.TurretGun`) "/Game/Gun/BP_DoubleBarreledGun.BP_DoubleBarreledGun_C")))

(event `Key|Three`
  (params (Key :type "Key Structure"))
  (:`Pressed`
    (`ChildActorComponent.SetChildActorClass` (`self.TurretGun`) "/Game/Gun/BP_LaserGun.BP_LaserGun_C")))

(event `Key|Four`
  (params (Key :type "Key Structure"))
  (:`Pressed`
    (`ChildActorComponent.SetChildActorClass` (`self.TurretGun`) "/Game/Gun/BP_ArcGun.BP_ArcGun_C")))

(fn `UserConstructionScript`)